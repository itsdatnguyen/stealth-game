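; BP_DoorKey is a key pickup that registers itself with its linked doors on BeginPlay and exposes its activated state.
; The player entering its sphere, sized by AquisitionRange at construction, activates it once.
; Activation alerts every CH_BasicEnemy: each updates the game mode's last known position and is flagged through its service to move there.
; Enemies not already aware also start an alert timer.
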(event `self.ReceiveBeginPlay`
  (for _array_element (`self.DoorsKeyCanOpen`)
    (`/Game/Game/Blueprint/Door.AssignToDoor` _array_element self)))

(event `self.CollisionSphere.OnComponentBeginOverlap`
  (params (OverlappedComponent :type "PrimitiveComponent Object Reference") (OtherActor :type "Actor Object Reference") (OtherComp :type "PrimitiveComponent Object Reference") (OtherBodyIndex :type Integer) (bFromSweep :type Boolean) (SweepResult :type "HitResult Structure (by ref)"))
  (bind _asgame_mode (cast `/Game/Game/Blueprint/Statics/Game_Mode` (`GameplayStatics.GetGameMode`) :!pure true))
  (if (== (`GameplayStatics.GetObjectClass` OtherActor) "/Game/Game/Blueprint/Player/PlayerCharacter.PlayerCharacter_C")
    (if (not (`self.Activated`))
      (set `self.Activated` true)
      (bind _outactors (`GameplayStatics.GetAllActorsOfClass` "/Game/Game/Blueprint/Enemy/CH_BasicEnemy.CH_BasicEnemy_C"))
      (for _array_element _outactors
        (bind _service (`/Game/Game/Blueprint/Enemy/CH_BasicEnemy.GetService` _array_element))
        (bind (_aggressive _aware) (`/Game/Game/Blueprint/Enemy/AI/TasksInUse/BP_BasicEnemyService.GetState` _service))
        (if _aware
          (`/Game/Game/Blueprint/Statics/Game_Mode.SetLastKnownPosition` _asgame_mode)
          (`/Game/Game/Blueprint/Enemy/AI/TasksInUse/BP_BasicEnemyService.SetFlagMoveToLastKnownLocation` _service)
          (else
            (`/Game/Game/Blueprint/Enemy/AI/TasksInUse/BP_BasicEnemyService.AlertTimer` _service)
            (`/Game/Game/Blueprint/Statics/Game_Mode.SetLastKnownPosition` _asgame_mode)
            (`/Game/Game/Blueprint/Enemy/AI/TasksInUse/BP_BasicEnemyService.SetFlagMoveToLastKnownLocation` _service)))))))

(fn `GetActivated`
  (returns (Activated :type Boolean))
  (return (`self.Activated`)))

(fn `UserConstructionScript`
  (`SphereComponent.SetSphereRadius` (`self.CollisionSphere`) (`self.AquisitionRange`) true))