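; Overhead follow camera actor that tracks the PlayerCharacter with stepped zoom and mouse-driven look-ahead.
; Zoom changes a clamped scroll count, which Tick eases into camera height around the starting ViewDistance.
; CalculatePosition interpolates toward the player's XY plus velocity lead and mouse sway, which grows as the camera zooms out.
; Each Tick also passes the camera's location to the player's CameraOffset before moving the actor.
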(event `self.ReceiveBeginPlay`
  (bind _outactors (`GameplayStatics.GetAllActorsOfClass` "/Game/Game/Blueprint/Player/PlayerCharacter.PlayerCharacter_C"))
  (for _array_element _outactors
    (set `self.Character Reference` _array_element)
    (set `self.NeutralViewDistance` (`self.ViewDistance`))))

(event `self.ReceiveTick`
  (params (DeltaSeconds :type "Float (single-precision)"))
  ;[1 1 1] Camera sway based on mouse location
  (`self.CameraInterpolation`)
  (bind _asplayer_character (cast `/Game/Game/Blueprint/Player/PlayerCharacter` (`self.Character Reference`)))
  (`/Game/Game/Blueprint/Player/PlayerCharacter.CameraOffset` _asplayer_character (`SceneComponent.K2_GetComponentLocation` (`self.CameraComponent`)))
  (bind _returnvalue (`self.CalculatePosition`))
  (`SceneComponent.K2_SetWorldLocation` _returnvalue))

(fn `CalculatePosition`
  (returns (ReturnValue :type "Vector Structure"))
  (bind (_locationx _locationy) (`WidgetLayoutLibrary.GetMousePositionScaledByDPI` (`GameplayStatics.GetPlayerController` 0)))
  (bind (_returnvalue_x _returnvalue_y) (`KismetMathLibrary.BreakVector` (`SceneComponent.K2_GetComponentLocation` (`self.Character Reference`))))
  (bind (_returnvalue_x_2 _returnvalue_y_2 _returnvalue_z) (`KismetMathLibrary.BreakVector` (`KismetMathLibrary.MakeVector` (* (`KismetMathLibrary.Lerp` (`self.LookUpMaxValue`) (`self.LookDownMaxValue`) (/ _locationy (`self.MaxMouseYValue`))) -1.0) (`KismetMathLibrary.Lerp` (`self.LookLeftMaxValue`) (`self.LookRightMaxValue`) (/ _locationx (`self.MaxMouseXValue`))))))
  (bind _returnvalue (`KismetMathLibrary.FInterpTo` (`self.ZoomLevel`) (`KismetMathLibrary.Lerp` 2.0 0.5 (/ (`KismetMathLibrary.Conv_IntToDouble` (+ (`self.ScrollAmount`) (`self.ZoomClamp`))) (`KismetMathLibrary.Conv_IntToDouble` (* (`self.ZoomClamp`) 2)))) (* (`GameplayStatics.GetWorldDeltaSeconds`) 2.0) 2.0))
  (set `self.ZoomLevel` _returnvalue)
  (return (`KismetMathLibrary.VInterpTo` (`SceneComponent.K2_GetComponentLocation` (`self.CameraComponent`)) (+ (+ (+ (`KismetMathLibrary.MakeVector` _returnvalue_x _returnvalue_y) (`KismetMathLibrary.MakeVector` 0.0 0.0 (`self.ViewDistance`))) (`KismetMathLibrary.MakeVector` (/ _returnvalue_x_2 _returnvalue) (/ _returnvalue_y_2 _returnvalue) _returnvalue_z)) (* (`self.GetVelocity` (`self.Character Reference`)) (* (`GameplayStatics.GetWorldDeltaSeconds`) 3.0))) (* (`GameplayStatics.GetWorldDeltaSeconds`) 5.0) 2.0)))

(fn `CameraInterpolation`
  (set `self.ViewDistance` (`KismetMathLibrary.FClamp` (`KismetMathLibrary.FInterpTo` (`self.ViewDistance`) (+ (* (`KismetMathLibrary.Conv_IntToDouble` (`self.ScrollAmount`)) (`self.ZoomAmount`)) (`self.NeutralViewDistance`)) (* (`GameplayStatics.GetWorldDeltaSeconds`) 5.0) 2.0) (- (`self.NeutralViewDistance`) (* (`KismetMathLibrary.Conv_IntToDouble` (`self.ZoomClamp`)) (`self.ZoomAmount`))) (+ (`self.NeutralViewDistance`) (* (`KismetMathLibrary.Conv_IntToDouble` (`self.ZoomClamp`)) (`self.ZoomAmount`))))))

(fn `UserConstructionScript`
  (`self.K2_SetActorRotation` (struct :`Pitch` 270.0)))

(fn `Zoom`
  (params (`True for Outward` :type Boolean))
  (if `True for Outward`
    (if (< (`self.ScrollAmount`) (`self.ZoomClamp`))
      (set `self.ScrollAmount` (+ (`self.ScrollAmount`) 1)))
    (elif (> (`self.ScrollAmount`) (* (`self.ZoomClamp`) -1))
      (set `self.ScrollAmount` (- (`self.ScrollAmount`) 1)))))