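; BP_Light_Parent is a light Blueprint, named as a parent class, that tracks when the player character is within its overlap area.
; On begin overlap it casts the other actor to PlayerCharacter and adds itself to that character's LightsOnPlayer array, guarded by a Find check.
; On end overlap it removes itself, so the character holds the list of lights currently affecting it.
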(event `self.ReceiveActorBeginOverlap`
  (params (OtherActor :type "Actor Object Reference"))
  (bind _asplayer_character (cast `/Game/Game/Blueprint/Player/PlayerCharacter` OtherActor))
  (bind _lightsonplayer (`/Game/Game/Blueprint/Player/PlayerCharacter.LightsOnPlayer` _asplayer_character))
  (if (== (`KismetArrayLibrary.Array_Find` _lightsonplayer null) -1)
    (`KismetArrayLibrary.Array_Add` _lightsonplayer self)))

(event `self.ReceiveActorEndOverlap`
  (params (OtherActor :type "Actor Object Reference"))
  (bind _asplayer_character (cast `/Game/Game/Blueprint/Player/PlayerCharacter` OtherActor))
  (`KismetArrayLibrary.Array_RemoveItem` (`/Game/Game/Blueprint/Player/PlayerCharacter.LightsOnPlayer` _asplayer_character) self))

(fn `UserConstructionScript`)