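; Thrown rock actor that distracts enemies by making noise where it lands.
; On BeginPlay it caches all CH_BasicEnemy actors, then destroys itself after a short delay.
; Each hit spawns a puff effect and tells the service of every cached enemy within a fixed radius to check the sound, passing the rock's location and itself.
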(event `self.ReceiveBeginPlay`
  (bind _outactors (`GameplayStatics.GetAllActorsOfClass` "/Game/Game/Blueprint/Enemy/CH_BasicEnemy.CH_BasicEnemy_C"))
  (set `self.EnemyArray` _outactors)
  (`KismetSystemLibrary.Delay` 5.0)
  (`self.K2_DestroyActor`))

(event `self.ReceiveHit`
  (params (MyComp :type "PrimitiveComponent Object Reference") (Other :type "Actor Object Reference") (OtherComp :type "PrimitiveComponent Object Reference") (bSelfMoved :type Boolean) (HitLocation :type "Vector Structure") (HitNormal :type "Vector Structure") (NormalImpulse :type "Vector Structure") (Hit :type "HitResult Structure (by ref)"))
  (`GameplayStatics.SpawnEmitterAtLocation` "/Game/Game/Particles/PS_Puff.PS_Puff" (`self.K2_GetActorLocation`))
  (for _array_element (`self.EnemyArray`)
    (if (<= (`KismetMathLibrary.VSize` (- (`self.K2_GetActorLocation`) (`self.K2_GetActorLocation` _array_element))) 600.0)
      (bind _service (`/Game/Game/Blueprint/Enemy/CH_BasicEnemy.GetService` _array_element))
      (`/Game/Game/Blueprint/Enemy/AI/TasksInUse/BP_BasicEnemyService.CheckSound` _service (`self.K2_GetActorLocation`) self))))

(fn `UserConstructionScript`)