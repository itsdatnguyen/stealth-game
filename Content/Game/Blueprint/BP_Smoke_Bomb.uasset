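; Smoke bomb actor that deploys a temporary smoke cloud on impact, affecting basic enemies inside it.
; A Cylinder hit spawns the smoke particles, makes SmokeCollision block Visibility and Camera traces, and flags overlapping CH_BasicEnemy actors as in smoke.
; Enemies are flagged only by that overlap query, not on later entry.
; A short timer calls DestroySelf, which clears the flag on enemies still overlapping and destroys the actor.
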(event `self.ReceiveBeginPlay`)

(event `self.Cylinder.OnComponentHit`
  (params (HitComponent :type "PrimitiveComponent Object Reference") (OtherActor :type "Actor Object Reference") (OtherComp :type "PrimitiveComponent Object Reference") (NormalImpulse :type "Vector Structure") (Hit :type "HitResult Structure (by ref)"))
  (bind _smoke_collision (`self.Smoke Collision`))
  (set `PrimitiveComponent.bGenerateOverlapEvents` true (`self.Smoke Collision`))
  (`self.CheckForOverlapping`)
  (`GameplayStatics.SpawnEmitterAtLocation` "/Game/Game/Particles/PS_Smoke_Bomb.PS_Smoke_Bomb" (`self.K2_GetActorLocation`))
  (`PrimitiveComponent.SetCollisionResponseToChannel` _smoke_collision "ECC_Visibility" "ECR_Block")
  (`PrimitiveComponent.SetCollisionResponseToChannel` _smoke_collision "ECC_Camera" "ECR_Block")
  (`KismetSystemLibrary.K2_SetTimer` null "DestroySelf" 5.0))

(fn `CheckForOverlapping`
  (for _array_element (`PrimitiveComponent.GetOverlappingActors` (`self.Smoke Collision`) "/Game/Game/Blueprint/Enemy/CH_BasicEnemy.CH_BasicEnemy_C")
    (`/Game/Game/Blueprint/Enemy/CH_BasicEnemy.SetInSmoke` (cast `/Game/Game/Blueprint/Enemy/CH_BasicEnemy` _array_element :!pure true) true))
  (return))

(fn `DestroySelf`
  (for _array_element (`PrimitiveComponent.GetOverlappingActors` (`self.Smoke Collision`) "/Game/Game/Blueprint/Enemy/CH_BasicEnemy.CH_BasicEnemy_C")
    (`/Game/Game/Blueprint/Enemy/CH_BasicEnemy.SetInSmoke` (cast `/Game/Game/Blueprint/Enemy/CH_BasicEnemy` _array_element :!pure true) false))
  (`self.K2_DestroyActor`)
  (return))

(fn `UserConstructionScript`)