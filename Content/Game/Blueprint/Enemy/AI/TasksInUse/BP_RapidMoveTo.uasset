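; Behavior tree task that sends a basic enemy toward the last known position held by the game mode.
; It runs from the task's Tick, caching the controlled CH_BasicEnemy and the game mode when the character reference is unset.
; It issues an AI MoveTo with a small acceptance radius and finishes successfully right away on the Then pin, without waiting for arrival.
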(event `self.ReceiveTick`
  (params (OwnerActor :type "Actor Object Reference") (DeltaSeconds :type "Float (single-precision)"))
  (if (== (`self.AICharacter`) null)
    (set `self.AICharacter` (cast `/Game/Game/Blueprint/Enemy/CH_BasicEnemy` (`Controller.K2_GetPawn` (cast `Controller` OwnerActor :!pure true)) :!pure true))
    (set `self.GameMode` (cast `/Game/Game/Blueprint/Statics/Game_Mode` (`GameplayStatics.GetGameMode`) :!pure true)))
  (bind _playerlastknownposition (`/Game/Game/Blueprint/Statics/Game_Mode.GetLastKnownPosition` (`self.GameMode`)))
  (`|AIMoveTo` (`self.AICharacter`) _playerlastknownposition null 10.0
    (:`then`
      (`self.FinishExecute` true))))