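; Behavior tree service for basic stealth enemies, handling player detection and writing alert states to the Blackboard.
; Each tick combines range, sight checks, a line trace and shadow/light rules to build an alert value from posture, distance, angle and exposure time, decaying it when sight is lost.
; Full alert triggers reinforcements, staggers awareness across other enemies through their services, and shares the player's last known position.
; Sound and touch functions raise suspicion.
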(event `MoveToLastKnownPosition`
  (if (`BTFunctionLibrary.GetBlackboardValueAsBool` (`self.MoveToLastKnownLocation`))
    (`BTFunctionLibrary.SetBlackboardValueAsBool` (`self.MoveToLastKnownLocation`))
    (`KismetSystemLibrary.Delay` 0.1))
  (`BTFunctionLibrary.SetBlackboardValueAsBool` (`self.MoveToLastKnownLocation`) true))

(event `SuspiciousTrue`
  ;[1 1 1] Miscellaneous Custom Functions
  (`BTFunctionLibrary.SetBlackboardValueAsBool` (`self.Suspicious`) true))

(event `self.ReceiveTick`
  (params (OwnerActor :type "Actor Object Reference") (DeltaSeconds :type "Float (single-precision)"))
  (bind _ascontroller (cast `Controller` OwnerActor :!pure true))
  (bind _isdead (`/Game/Game/Blueprint/Enemy/CH_BasicEnemy.IsDead` (`self.AI Character Reference`)))
  (bind _asch_basic_enemy (cast `/Game/Game/Blueprint/Enemy/CH_BasicEnemy` (`Controller.K2_GetPawn` _ascontroller) :!pure true))
  (if (not (!= (`self.AI Controller Reference`) null))
    ;[1 1 1] Ran Only Once At Start
    (set `self.AI Controller Reference` _ascontroller)
    (set `/Game/Game/Blueprint/Enemy/CH_BasicEnemy.Service` self _asch_basic_enemy)
    (bind _output_get (set `self.AI Character Reference` _asch_basic_enemy))
    (bind _player (`/Game/Game/Blueprint/Enemy/CH_BasicEnemy.GetPlayer` _output_get))
    (set `self.PlayerCharacter` _player)
    (bind _outactors (`GameplayStatics.GetAllActorsOfClass` "/Game/Game/Blueprint/Enemy/CH_BasicEnemy.CH_BasicEnemy_C"))
    (set `self.EnemyArray` _outactors)
    (bind _detectionwidget (`/Game/Game/Blueprint/Enemy/CH_BasicEnemy.GetDetectionWidget` _asch_basic_enemy))
    (set `self.DetectionHUD` _detectionwidget)
    (set `self.GameMode` (cast `/Game/Game/Blueprint/Statics/Game_Mode` (`GameplayStatics.GetGameMode`) :!pure true))
    (if (`/Game/Game/Blueprint/Statics/Game_Mode.DebugMode` (`self.GameMode`))
      (set `self.DebugEnum` "ForOneFrame")
      (else
        (set `self.DebugEnum` "None")))
    (if (`.bSuccess` (cast `/Game/Game/Blueprint/Statics/GameModeHuntDoors` (`self.GameMode`) :!pure true))
      (`self.SetAwareToTrue`)
      (`self.SetFlagMoveToLastKnownLocation`)))
  (`BTFunctionLibrary.SetBlackboardValueAsBool` (`self.IsDead`) _isdead)
  (if _isdead
    _
    (elif (<= (`KismetMathLibrary.VSize` (- (`Actor.K2_GetActorLocation` (`self.AI Character Reference`)) (`Actor.K2_GetActorLocation` (`self.PlayerCharacter`)))) (`self.DetectionRadius`))
      (bind (_playerinvisioncone _playerinlightcone _playerinfootcheck) (`/Game/Game/Blueprint/Enemy/CH_BasicEnemy.CheckIfPlayerIsInSight` (`self.AI Character Reference`)))
      (if (or _playerinvisioncone _playerinfootcheck)
        (bind _outhit (`KismetSystemLibrary.LineTraceSingle` :`Start` (+ (`Actor.K2_GetActorLocation` (`self.AI Character Reference`)) (0.0 0.0 75.0)) :`End` (`SceneComponent.K2_GetComponentLocation` (`/Game/Game/Blueprint/Player/PlayerCharacter.Invisibillity Sphere` (`self.PlayerCharacter`))) :`TraceChannel` "TraceTypeQuery2" :`DrawDebugType` (`self.DebugEnum`)))
        (if (== (`/Game/Game/Blueprint/Player/PlayerCharacter.Invisibillity Sphere` (`self.PlayerCharacter`)) (`.HitComponent` (`GameplayStatics.BreakHitResult` _outhit)))
          (if (or (not (`/Game/Game/Blueprint/Player/PlayerCharacter.InShadow` (`self.PlayerCharacter`))) _playerinfootcheck _playerinlightcone)
            (`/Game/Game/Blueprint/Player/PlayerCharacter.SetInLight` (`self.PlayerCharacter`))
            (if (> (`self.AlertValue`) 100.0)
              _
              (elif (`BTFunctionLibrary.GetBlackboardValueAsBool` (`self.Aggressive`))
                (set `self.AlertValue` (+ (`self.AlertValue`) (`self.AggressiveModifier`)))
                (`self.CalculateDetection`)
                (else
                  (`self.CalculateDetection`))))
            (if (>= (`self.AlertValue`) 100.0)
              (`|ExecutionSequence`
                (:`then_0`
                  (if (not (`BTFunctionLibrary.GetBlackboardValueAsBool` (`self.Set Aware`)))
                    (`self.AlertAll`)
                    (`self.AlertReinforcements`))
                  (`self.SawTarget`))
                (:`then_1`
                  (goto _label :!via `Open`)))))
          (else
            ;[1 1 1] If raycast missed
            (`self.DecayDetection`)
            (set `self.NumberOfTicksInSight` 0)
            (`BTFunctionLibrary.SetBlackboardValueAsBool` (`self.AquiredTarget`))
            (`/Engine/EditorBlueprintResources/StandardMacros.Gate` true :!label _label
              (:`Exit`
                (`|ExecutionSequence`
                  (:`then_0`
                    (`KismetSystemLibrary.Delay` 0.4)
                    (`self.SetLastSeenDirection`))
                  (:`then_1`
                    (goto _label :!via `Close`)))))))
        (else
          (`self.DecayDetection` :!label _label_2)
          (`BTFunctionLibrary.SetBlackboardValueAsBool` (`self.AquiredTarget`))))
      (else
        (goto _label_2)))))

(event `SawTarget`
  (bind _gamemode (`self.GameMode`))
  (bind _playercharacter (`self.PlayerCharacter`))
  ;[1 1 1] Saw Target: Runs every tick the enemy sees the player
  (`|ExecutionSequence`
    (:`then_0`
      ;[1 1 1] Runs only once when the enemy first chases the player
      (`/Engine/EditorBlueprintResources/StandardMacros.Gate` false :!label _label_3
        (:`Exit`
          (`/Game/Game/Blueprint/Enemy/CH_BasicEnemy.SetLight` (`self.AI Character Reference`) true)
          (set `self.AwareSightModifier` (`self.AwareSightNumber`))
          (`BTFunctionLibrary.SetBlackboardValueAsBool` (`self.Set Aware`) true)
          (goto _label_3 :!via `Close`))))
    (:`then_1`
      (`/Game/Game/Blueprint/Statics/Game_Mode.SetLastKnownPosition` (`self.GameMode`))
      (message `/Game/Game/Blueprint/Statics/BP_CharacterInterface.Set Move Max` (`self.AI Character Reference`))
      (set `self.JustSawTarget` true)
      (`BTFunctionLibrary.SetBlackboardValueAsBool` (`self.Suspicious`))
      (`BTFunctionLibrary.SetBlackboardValueAsBool` (`self.PlayerRewindWhileInSight`))
      (`BTFunctionLibrary.SetBlackboardValueAsBool` (`self.AquiredTarget`) true)
      (`BTFunctionLibrary.SetBlackboardValueAsBool` (`self.Aggressive`) true)
      (`|ExecutionSequence`
        (:`then_0`
          (`KismetSystemLibrary.Delay` (+ (`KismetMathLibrary.RandomFloatInRange` -1.0 1.0) 2.0))
          (`self.SetAllToFindCharacter`))
        (:`then_1`
          (`/Game/Game/Blueprint/Statics/Game_Mode.SetGhostParameters` _gamemode (`Actor.K2_GetActorLocation` _playercharacter) (`KismetMathLibrary.ComposeRotators` (`Actor.K2_GetActorRotation` _playercharacter) (struct :`Yaw` -90.0)))
          (`KismetSystemLibrary.RetriggerableDelay` 1.0)
          (`/Game/Game/Blueprint/Statics/Game_Mode.SetGhostIndicator` _gamemode))
        (:`then_2`
          (`KismetSystemLibrary.RetriggerableDelay` 1.5)
          (set `self.JustSawTarget` false))))))

(fn `AlertAll`
  (for _array_element (`self.EnemyArray`)
    (bind _service (`/Game/Game/Blueprint/Enemy/CH_BasicEnemy.GetService` _array_element))
    (bind (_aggressive _aware) (`self.GetState` _service))
    (if (not _aware)
      (`self.AlertTimer` _service)
      (`self.AlertTimer` _service))))

(fn `AlertReinforcements`
  (message `/Game/Game/Blueprint/Statics/BP_Gamemode_Interface.ActivateReinforcements` (`GameplayStatics.GetGameMode`)))

(fn `AlertTimer`
  (`KismetSystemLibrary.K2_SetTimer` null "SetAwareToTrue" (+ 2.0 (`KismetMathLibrary.RandomFloatInRange` -1.5 1.5))))

(fn `CalculateDetection`
  (locals (ShadowModifier :type "Float (double-precision)" :default 0.08) (AddedValue :type "Float (double-precision)") (InLightConeModifier :type "Float (double-precision)" :default 0.05) (DistanceMultiplier :type "Float (double-precision)" :default 0.1) (RepeatMultiplier :type "Float (double-precision)" :default 0.01) (SightDistanceAlertModifier :type "Float (double-precision)" :default 3000.0) (Yaw :type "Float (double-precision)") (CrouchedModifier :type "Float (double-precision)" :default 0.06))
  (bind _ai_character_reference (`self.AI Character Reference`))
  (set `local.AddedValue` 0.0)
  (set `self.NumberOfTicksInSight` (+ (`self.NumberOfTicksInSight`) 1))
  ;[1 1 1] Added value if player is not crouched
  (bind _iscrouched (`/Game/Game/Blueprint/Player/PlayerCharacter.GetMovementModifiers` (`self.PlayerCharacter`)))
  (if (not _iscrouched)
    (set `local.AddedValue` (+ (`local.AddedValue`) (`local.CrouchedModifier`))))
  ;[1 1 1] Shadow modifier is added if player is not in shadow
  (bind (_isinshadow _isinlight) (`/Game/Game/Blueprint/Player/PlayerCharacter.GetSightModifiers` (`self.PlayerCharacter`)))
  (if (not _isinshadow)
    (set `local.AddedValue` (+ (`local.ShadowModifier`) (`local.AddedValue`))))
  ;[1 1 1] Light cone modifier is added if player is in a enemy light cone or light actor
  (if _isinlight
    (set `local.AddedValue` (+ (`local.InLightConeModifier`) (`local.AddedValue`))))
  (bind _yaw (`/Game/Game/Blueprint/Enemy/CH_BasicEnemy.GetAimOffset` (`self.AI Character Reference`)))
  (set `local.Yaw` _yaw)
  (bind _output_get (set `local.AddedValue` (* (+ (* (`local.DistanceMultiplier`) (`KismetMathLibrary.Lerp` 40.0 0.0 (/ (`KismetMathLibrary.VSize` (- (`Actor.K2_GetActorLocation` (`self.AI Character Reference`)) (`Actor.K2_GetActorLocation` (`self.PlayerCharacter`)))) (`local.SightDistanceAlertModifier`)))) (* (`local.RepeatMultiplier`) (/ (`KismetMathLibrary.MultiplyMultiply_FloatFloat` (`KismetMathLibrary.Conv_IntToDouble` (`self.NumberOfTicksInSight`)) 2.0) 10.0)) (`self.SuspiciousModifier`) (`self.AwareSightModifier`) (`local.AddedValue`)) (`KismetMathLibrary.Lerp` 1.2 0.2 (/ (`KismetMathLibrary.Abs` (- (.yaw (`KismetMathLibrary.NormalizedDeltaRotator` (`KismetMathLibrary.FindLookAtRotation` (`Actor.K2_GetActorLocation` _ai_character_reference) (`Actor.K2_GetActorLocation` (`self.PlayerCharacter`))) (`Actor.K2_GetActorRotation` _ai_character_reference))) (`local.Yaw`))) 40.0)))))
  ;[1 1 1] Finally the accrued amount is added to the alert value and multiplied by Detection Level
  (set `self.AlertValue` (+ (* (`local.AddedValue`) (+ (/ (`KismetMathLibrary.Conv_IntToDouble` (`self.DetectionLevel`)) 4.0) 1.0)) (`self.AlertValue`))))

(fn `CheckSound`
  (params (SoundLocation :type "Vector Structure" :default (0.0 0.0 0.0)) (RockActor :type "Actor Object Reference"))
  (`BTFunctionLibrary.SetBlackboardValueAsVector` (`self.SoundLocation`) SoundLocation)
  (if (`BTFunctionLibrary.GetBlackboardValueAsBool` (`self.Suspicious`))
    (`BTFunctionLibrary.SetBlackboardValueAsBool` (`self.Suspicious`))
    (`KismetSystemLibrary.K2_SetTimer` null "SuspiciousTrue" 0.02)
    (else
      (`BTFunctionLibrary.SetBlackboardValueAsBool` (`self.Suspicious`) true)))
  (`self.SetSuspiciousModifier` true)
  (`BTFunctionLibrary.SetBlackboardValueAsObject` (`self.SearchActor`) (cast `/Game/Game/Blueprint/Rock` RockActor :!pure true)))

(fn `DecayDetection`
  (if (> (`self.AlertValue`) 0.0)
    (set `self.AlertValue` (- (`self.AlertValue`) 0.75))
    (else
      (set `self.AlertValue` 0.0)))
  (return))

(fn `GetActionKeys`
  (returns (`Player Rewind` :type Boolean) (`Is Moving To Last Known Location` :type Boolean))
  (return (`BTFunctionLibrary.GetBlackboardValueAsBool` (`self.PlayerRewindWhileInSight`)) (`BTFunctionLibrary.GetBlackboardValueAsBool` (`self.MoveToLastKnownLocation`))))

(fn `GetEnemyArray`
  (returns (EnemyArray :type "Array of /Game/Game/Blueprint/Enemy/CH_BasicEnemy Object Reference"))
  (return (`self.EnemyArray`)))

(fn `GetState`
  (returns (Aggressive :type Boolean) (Aware :type Boolean) (Suspicious :type Boolean) (AquiredTarget :type Boolean))
  (return (`BTFunctionLibrary.GetBlackboardValueAsBool` (`self.Aggressive`)) (`BTFunctionLibrary.GetBlackboardValueAsBool` (`self.Set Aware`)) (`BTFunctionLibrary.GetBlackboardValueAsBool` (`self.Suspicious`)) (`BTFunctionLibrary.GetBlackboardValueAsBool` (`self.AquiredTarget`))))

(fn `MakeHUD`
  (if (== (`self.DetectionHUD`) null)
    (bind _returnvalue (`|CreateWidget` "/Game/Game/Blueprint/UI/EnemyDetectionHUD.EnemyDetectionHUD_C" (`GameplayStatics.GetPlayerController` 0)))
    (bind _output_get (set `self.DetectionHUD` _returnvalue))
    (`UserWidget.AddToViewport` _output_get 0)))

(fn `SetAllToFindCharacter`
  (for _array_element (`self.EnemyArray`)
    (bind _service (`/Game/Game/Blueprint/Enemy/CH_BasicEnemy.GetService` _array_element))
    (`self.MoveToLastKnownPosition` _service)))

(fn `SetAquiredTarget`
  (params (AquiredTarget :type Boolean))
  (`BTFunctionLibrary.SetBlackboardValueAsBool` (`self.AquiredTarget`) AquiredTarget))

(fn `SetAware`
  (params (Boolean :type Boolean))
  (`BTFunctionLibrary.SetBlackboardValueAsBool` (`self.Set Aware`) Boolean))

(fn `SetAwareToTrue`
  (`BTFunctionLibrary.SetBlackboardValueAsBool` (`self.Set Aware`) true)
  (`/Game/Game/Blueprint/Enemy/CH_BasicEnemy.SetLight` (`self.AI Character Reference`) true)
  (`/Game/Game/Blueprint/Enemy/CH_BasicEnemy.Set Move Min` (`self.AI Character Reference`))
  (set `self.AwareSightModifier` (`self.AwareSightNumber`))
  (`self.MoveToLastKnownPosition`))

(fn `SetFlagMoveToLastKnownLocation`
  (`BTFunctionLibrary.SetBlackboardValueAsBool` (`self.MoveToLastKnownLocation`))
  (`KismetSystemLibrary.K2_SetTimer` self "MoveToLocation" 0.1))

(fn `SetLastSeenDirection`
  (locals (Angle :type "Float (double-precision)"))
  (bind _ai_character_reference (`self.AI Character Reference`))
  (bind _lastseendirection (`self.LastSeenDirection`))
  (bind _playercharacter (`self.PlayerCharacter`))
  (bind _yaw (`/Game/Game/Blueprint/Enemy/CH_BasicEnemy.GetAimOffset` (`self.AI Character Reference`)))
  (if (< (- (.yaw (`KismetMathLibrary.NormalizedDeltaRotator` (`KismetMathLibrary.FindLookAtRotation` (`Actor.K2_GetActorLocation` _ai_character_reference) (+ (`Actor.K2_GetActorLocation` _playercharacter) (`Actor.GetVelocity` _playercharacter))) (`Actor.K2_GetActorRotation` _ai_character_reference))) _yaw) 0.0)
    (`BTFunctionLibrary.SetBlackboardValueAsBool` _lastseendirection true)
    (else
      (`BTFunctionLibrary.SetBlackboardValueAsBool` _lastseendirection))))

(fn `SetPlayerRewindWhileInSight`
  (`BTFunctionLibrary.SetBlackboardValueAsBool` (`self.PlayerRewindWhileInSight`) true))

(fn `SetSuspiciousModifier`
  (params (Boolean :type Boolean))
  (if Boolean
    (set `self.SuspiciousModifier` 5.0)
    (else
      (set `self.SuspiciousModifier` 0.0))))

(fn `TouchedPlayer`
  (if (not (and (`BTFunctionLibrary.GetBlackboardValueAsBool` (`self.Aggressive`)) (`BTFunctionLibrary.GetBlackboardValueAsBool` (`self.Suspicious`))))
    (`BTFunctionLibrary.SetBlackboardValueAsBool` (`self.Suspicious`) true)
    (`BTFunctionLibrary.SetBlackboardValueAsVector` (`self.SoundLocation`) (`Actor.K2_GetActorLocation` (`self.PlayerCharacter`)))
    (`BTFunctionLibrary.SetBlackboardValueAsObject` (`self.SearchActor`))))