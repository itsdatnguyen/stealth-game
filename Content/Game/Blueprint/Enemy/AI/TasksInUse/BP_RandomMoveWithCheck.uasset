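; Behavior tree task that moves an enemy AI pawn to a random navigable point, used for wandering.
; It picks a point within a maximum radius and fails unless the nav path length lies between the minimum and maximum limits.
; After the move succeeds or fails, it randomly either waits briefly and reissues the move to the stored location, or finishes successfully.
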(event `self.ReceiveExecute`
  (params (OwnerActor :type "Actor Object Reference"))
  (bind _returnvalue (`Controller.K2_GetPawn` (`self.AIController`)))
  (if (== (`self.AIController`) null)
    (set `self.AIController` (cast `AIController` OwnerActor :!pure true)))
  (bind _output_get (set `self.Location` (`NavigationSystem.GetRandomPointInNavigableRadius` (`Actor.K2_GetActorLocation` _returnvalue) (`self.MoveMaximum`))))
  (bind _pathlength (`NavigationSystem.GetPathLength` (`Actor.K2_GetActorLocation` _returnvalue) _output_get))
  (if (and (< _pathlength (`self.MoveMaximum`)) (> _pathlength (`self.MoveMinimum`)))
    (`|AIMoveTo` _returnvalue (`self.Location`) null 50.0 :!label _label
      (:`OnSuccess`
        _)
      (:`OnFail`
        _))
    (if (== (`KismetMathLibrary.RandomInteger` 3) 0)
      (`KismetSystemLibrary.Delay` (+ (`KismetMathLibrary.RandomFloatInRange` -0.6 0.6) 0.8))
      (goto _label)
      (else
        (`self.FinishExecute` true)))
    (else
      (`self.FinishExecute` false))))