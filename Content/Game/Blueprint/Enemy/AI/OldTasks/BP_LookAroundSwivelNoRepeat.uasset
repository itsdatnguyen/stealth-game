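; Old behavior tree task that makes a CH_BasicEnemy look around once, swiveling its sight to both sides in random order.
; The Turner event steps yaw through ChangeSight on a timed loop, using a quadratic curve around the midpoint to vary turn speed.
; Each turn gets a random step count and is followed by a separately randomized delay, then the task finishes successfully.
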(event `self.ReceiveExecute`
  (params (OwnerActor :type "Actor Object Reference"))
  (bind _returnvalue (`KismetMathLibrary.RandomIntegerInRange` (`self.MinInt`) (`self.MaxInt`)))
  (bind _returnvalue_2 (`KismetMathLibrary.RandomIntegerInRange` (`self.MinInt`) (`self.MaxInt`)))
  (bind _returnvalue_3 (`KismetMathLibrary.RandomIntegerInRange` (`self.MinInt`) (`self.MaxInt`)))
  (bind _returnvalue_4 (`KismetMathLibrary.RandomIntegerInRange` (`self.MinInt`) (`self.MaxInt`)))
  (bind _asaicontroller (cast `AIController` OwnerActor))
  (bind _asch_basic_enemy (cast `/Game/Game/Blueprint/Enemy/CH_BasicEnemy` (`Controller.K2_GetPawn` _asaicontroller)))
  (set `self.AICharacter` _asch_basic_enemy)
  (if (== (`KismetMathLibrary.RandomInteger` 2) 0)
    (`self.Turner` _returnvalue_3 (* (`self.TurnAmount`) -1.0))
    (`KismetSystemLibrary.Delay` (* (`self.Delay`) (`KismetMathLibrary.Conv_IntToDouble` _returnvalue_3) (`self.MoreDelay`)))
    (`self.Turner` _returnvalue_4 (`self.TurnAmount`))
    (`KismetSystemLibrary.Delay` (* (`KismetMathLibrary.Conv_IntToDouble` _returnvalue_4) (`self.Delay`) (`self.MoreDelay`)))
    (else
      (`self.Turner` _returnvalue (`self.TurnAmount`))
      (`KismetSystemLibrary.Delay` (* (`self.Delay`) (`KismetMathLibrary.Conv_IntToDouble` _returnvalue) (`self.MoreDelay`)))
      (`self.Turner` _returnvalue_2 (* (`self.TurnAmount`) -1.0))
      (`KismetSystemLibrary.Delay` (* (`KismetMathLibrary.Conv_IntToDouble` _returnvalue_2) (`self.Delay`) (`self.MoreDelay`)))))
  (`self.FinishExecute` true))

(event `Turner`
  (params (`Last Index` :type Integer :default 0) (`Turn Amount` :type "Float (double-precision)" :default 0.0))
  (bind _index (`self.Index`))
  (bind _aicharacter (`self.AICharacter`))
  (bind _yaw (`/Game/Game/Blueprint/Enemy/CH_BasicEnemy.Yaw` _aicharacter))
  ;[1 1 1] Turner Function
  (set `self.LookTimeConstant` (/ (`KismetMathLibrary.Conv_IntToDouble` `Last Index`) 2.0))
  (set `self.Index` 0)
  (if (<= _index `Last Index`) :!label _label
    (set `self.Index` (+ _index 1))
    (`/Game/Game/Blueprint/Enemy/CH_BasicEnemy.ChangeSight` _aicharacter (+ (* (+ (* (`self.Multiplier`) (`KismetMathLibrary.MultiplyMultiply_FloatFloat` (- (`KismetMathLibrary.Conv_IntToDouble` (`self.Index`)) (`self.LookTimeConstant`)) 2.0)) (`self.LookSpeedConstant`)) `Turn Amount`) _yaw) 0.0)
    (`KismetSystemLibrary.Delay` (`self.Delay`))
    (goto _label)
    (else
      (`/Game/Game/Blueprint/Enemy/CH_BasicEnemy.ChangeSight` _aicharacter _yaw 0.0))))