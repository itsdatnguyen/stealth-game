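; Legacy behavior tree task that gives an enemy AI a random search destination.
; On execute it fetches the character through the AI controller via interface messages and checks its state.
; If the state check fails it aborts; otherwise it writes a random navigable point near the character to the Destination blackboard key and finishes successfully.
; Tick repeats the state check to abort, and the debug prints are unreachable.
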(event `self.ReceiveTick`
  (params (OwnerActor :type "Actor Object Reference") (DeltaSeconds :type "Float (single-precision)"))
  (message `/Game/Game/Blueprint/Statics/BP_CharacterInterface.Get State` (`self.Character Reference`))
  (if false
    (`self.FinishAbort`)))

(event `self.ReceiveExecute`
  (params (OwnerActor :type "Actor Object Reference"))
  (bind _returnvalue (`AIBlueprintHelperLibrary.GetAIController` OwnerActor))
  (bind _output_get (set `self.Character Controller Reference` _returnvalue))
  (message `/Game/Game/Blueprint/Statics/BP_CharacterInterface.Get Character Reference` _output_get)
  (bind _output_get_2 (set `self.Character Reference` null))
  (message `/Game/Game/Blueprint/Statics/BP_CharacterInterface.Get State` _output_get_2)
  (bind _output_get_3 (set `self.State` false))
  (if _output_get_3
    (`self.FinishAbort`)
    (else
      (`BTFunctionLibrary.SetBlackboardValueAsVector` (`self.Destination`) (`NavigationSystem.GetRandomPointInNavigableRadius` (`Actor.K2_GetActorLocation` (`self.Character Reference`)) 1024.0))
      (`self.FinishExecute` true))))