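; Behavior tree task that sends a CH_BasicEnemy walking to a random point ahead of it.
; It offsets the enemy's location along the blackboard forward and right vectors with random spread, stores the result in ForwardSearchVector, and runs AIMoveTo toward it.
; On success or failure it calls SetMoveMinMessage on the pawn, finishes with the matching result, then clears the Aggressive key.
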(event `self.ReceiveExecute`
  (params (OwnerActor :type "Actor Object Reference"))
  (bind _aicharacter (`self.AICharacter`))
  (bind _returnvalue (`BTFunctionLibrary.GetBlackboardValueAsVector` (`self.ForwardDirectionVector`)))
  (bind _ascontroller (cast `Controller` OwnerActor))
  (bind _output_get (set `self.AICharacter` (`Controller.K2_GetPawn` _ascontroller)))
  (bind _asch_basic_enemy (cast `/Game/Game/Blueprint/Enemy/CH_BasicEnemy` _output_get))
  (`BTFunctionLibrary.SetBlackboardValueAsVector` (`self.ForwardSearchVector`) (+ (`Actor.K2_GetActorLocation` _asch_basic_enemy) (+ (* _returnvalue 400.0) (* (* _returnvalue (`KismetMathLibrary.RandomFloatInRange` -1.0 1.0)) 300.0)) (* (* (`BTFunctionLibrary.GetBlackboardValueAsVector` (`self.RightDirectionVector`)) (`KismetMathLibrary.RandomFloatInRange` -1.0 1.0)) 500.0)))
  (`|AIMoveTo` _asch_basic_enemy (`BTFunctionLibrary.GetBlackboardValueAsVector` (`self.ForwardSearchVector`)) null 50.0
    (:`OnSuccess`
      (message `/Game/Game/Blueprint/Statics/BP_CharacterInterface.Set Move Min` _aicharacter)
      (`self.FinishExecute` true))
    (:`OnFail`
      (message `/Game/Game/Blueprint/Statics/BP_CharacterInterface.Set Move Min` _aicharacter)
      (`self.FinishExecute` false)))
  (`BTFunctionLibrary.SetBlackboardValueAsBool` (`self.Aggressive`)))