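; Behavior Tree task, in an OldTasks folder, that makes an AI enemy look around by rotating its character.
; It turns one way then the other in random order, with randomized step counts and pauses, and has a one-in-three chance to repeat before finishing.
; The Turner event applies yaw in delayed increments, sized by a quadratic curve around the turn's midpoint.
; The PlayerController variable actually holds the AI's character reference.
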(event `self.ReceiveExecute`
  (params (OwnerActor :type "Actor Object Reference"))
  (bind _returnvalue (`KismetMathLibrary.RandomIntegerInRange` (`self.MinInt`) (`self.MaxInt`)))
  (bind _returnvalue_2 (`KismetMathLibrary.RandomIntegerInRange` (`self.MinInt`) (`self.MaxInt`)))
  (bind _returnvalue_3 (`KismetMathLibrary.RandomIntegerInRange` (`self.MinInt`) (`self.MaxInt`)))
  (bind _returnvalue_4 (`KismetMathLibrary.RandomIntegerInRange` (`self.MinInt`) (`self.MaxInt`)))
  (bind _asaicontroller (cast `AIController` OwnerActor))
  (bind _actor_reference (message `/Game/Game/Blueprint/Statics/BP_CharacterInterface.Get Character Reference` _asaicontroller))
  (set `self.Player Controller` _actor_reference)
  (if (== (`KismetMathLibrary.RandomInteger` 2) 0) :!label _label
    (`self.Turner` _returnvalue_3 (* (`self.TurnAmount`) -1.0))
    (`KismetSystemLibrary.Delay` (* (`self.Delay`) (`KismetMathLibrary.Conv_IntToDouble` _returnvalue_3) (`self.MoreDelay`)))
    (`self.Turner` _returnvalue_4 (`self.TurnAmount`))
    (`KismetSystemLibrary.Delay` (* (`KismetMathLibrary.Conv_IntToDouble` _returnvalue_4) (`self.Delay`) (`self.MoreDelay`)))
    (else
      (`self.Turner` _returnvalue (`self.TurnAmount`))
      (`KismetSystemLibrary.Delay` (* (`self.Delay`) (`KismetMathLibrary.Conv_IntToDouble` _returnvalue) (`self.MoreDelay`)))
      (`self.Turner` _returnvalue_2 (* (`self.TurnAmount`) -1.0))
      (`KismetSystemLibrary.Delay` (* (`KismetMathLibrary.Conv_IntToDouble` _returnvalue_2) (`self.Delay`) (`self.MoreDelay`)))))
  (if (== (`KismetMathLibrary.RandomInteger` 3) 0)
    (`KismetSystemLibrary.Delay` (+ (`KismetMathLibrary.RandomFloatInRange` -0.6 0.6) 0.8))
    (goto _label)
    (else
      (`self.FinishExecute` true))))

(event `Turner`
  (params (`Last Index` :type Integer :default 0) (`Turn Amount` :type "Float (double-precision)" :default 0.0))
  (bind _index (`self.Index`))
  ;[1 1 1] Turner Function
  (set `self.LookTimeConstant` (/ (`KismetMathLibrary.Conv_IntToDouble` `Last Index`) 2.0))
  (set `self.Index` 0)
  (if (<= _index `Last Index`) :!label _label_2
    (set `self.Index` (+ _index 1))
    (`KismetSystemLibrary.Delay` (`self.Delay`))
    (`Actor.K2_SetActorRotation` (`self.Player Controller`) (`KismetMathLibrary.ComposeRotators` (`Actor.K2_GetActorRotation` (`self.Player Controller`)) (`KismetMathLibrary.MakeRotator` 0.0 0.0 (* (+ (* (`self.Multiplier`) (`KismetMathLibrary.MultiplyMultiply_FloatFloat` (- (`KismetMathLibrary.Conv_IntToDouble` (`self.Index`)) (`self.LookTimeConstant`)) 2.0)) (`self.LookSpeedConstant`)) `Turn Amount`))) false)
    (goto _label_2)))