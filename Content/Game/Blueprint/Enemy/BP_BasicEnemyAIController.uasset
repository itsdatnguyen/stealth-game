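; BP_BasicEnemyAIController is the AI controller for a basic enemy.
; On BeginPlay it starts the BasicAIBehavior behavior tree, which carries the enemy's logic outside this Blueprint.
; GetCharacterReference returns the controlled pawn.
; The remaining functions for state, perception, movement limits, projectile hits and kill checks are stubs that return default values.
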(event `self.ReceiveBeginPlay`
  (`self.RunBehaviorTree` "/Game/Game/Blueprint/Enemy/AI/BasicAIBehavior.BasicAIBehavior"))

(fn `CheckForKill`
  (params (`Impact Normal` :type "Vector Structure") (`Impact Location` :type "Vector Structure"))
  (returns (NewParam :type Boolean))
  (return false))

(fn `Get Character Reference`
  (returns (`Actor Reference` :type "Pawn Object Reference"))
  (return (`self.K2_GetPawn`)))

(fn `Get Last Seen Location`
  (returns (`Last Seen Location` :type "Vector Structure"))
  (return (0.0 0.0 0.0)))

(fn `Get Location`
  (params (Actor :type "Actor Object Reference"))
  (returns (Lcoation :type "Vector Structure"))
  (return (0.0 0.0 0.0)))

(fn `Get State`
  (returns (Touched :type Boolean))
  (return false))

(fn `Get Timer`
  (returns (Time :type "Float (double-precision)"))
  (return 0.0))

(fn `Get Visibility`
  (params (Actor :type "Actor Object Reference"))
  (returns (`Visibility Value` :type "Float (double-precision)"))
  (return 0.0))

(fn `HitByProjectile`
  (params (`Hit Value` :type "Float (double-precision)"))
  (returns (NewParam1 :type "Float (double-precision)"))
  (return 0.0))

(fn `Set Move Max`
  (returns (NewParam :type Boolean))
  (return false))

(fn `Set Move Min`
  (returns (NewParam :type Boolean))
  (return false))

(fn `UserConstructionScript`)