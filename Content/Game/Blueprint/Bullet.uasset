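; Bullet projectile actor that damages player characters it hits and destroys itself after a five-second lifetime.
; On Hit, it casts to PlayerCharacter and, only for capsule hits, sends fixed damage, passes impact data to a kill check, then destroys itself.
; Other hits leave the bullet alive until the timer expires.
; A disconnected branch holds unused CH_BasicEnemy logic with bone-name headshot damage.
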(event `self.ReceiveBeginPlay`
  (`KismetSystemLibrary.Delay` 5.0)
  (`self.K2_DestroyActor`))

(event `self.ReceiveHit`
  (params (MyComp :type "PrimitiveComponent Object Reference") (Other :type "Actor Object Reference") (OtherComp :type "PrimitiveComponent Object Reference") (bSelfMoved :type Boolean) (HitLocation :type "Vector Structure") (HitNormal :type "Vector Structure") (NormalImpulse :type "Vector Structure") (Hit :type "HitResult Structure (by ref)"))
  (bind (_bblockinghit _binitialoverlap _time _location _impactpoint _normal _impactnormal _physmat _hitactor _hitcomponent _hitbonename) (`GameplayStatics.BreakHitResult` Hit))
  (set `self.OtherComp` OtherComp)
  (set `self.HitActor` _hitactor)
  (bind _asplayer_character (cast `/Game/Game/Blueprint/Player/PlayerCharacter` (`self.HitActor`)))
  (if (== (`Character.CapsuleComponent` _asplayer_character) _hitcomponent)
    (message `/Game/Game/Blueprint/Statics/BP_CharacterInterface.HitByProjectile` _asplayer_character 30.0)
    (`/Game/Game/Blueprint/Statics/BP_CharacterInterface.CheckForKill` _asplayer_character _impactnormal _impactpoint)
    (`self.K2_DestroyActor`)))

(fn `UserConstructionScript`)