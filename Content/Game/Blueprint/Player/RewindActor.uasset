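; RewindActor is an actor that marks the player character's current rewind location with a spinning, trailing presence.
; On BeginPlay it finds and stores a PlayerCharacter from the world.
; Each Tick it eases toward that character's RewindCurrentLocation with VInterpTo.
; It also accumulates elapsed time to drive a continuous rotation at a different rate on each axis.
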(event `self.ReceiveBeginPlay`
  (bind _outactors (`GameplayStatics.GetAllActorsOfClass` "/Game/Game/Blueprint/Player/PlayerCharacter.PlayerCharacter_C"))
  (for _array_element _outactors
    (set `self.PlayerCharacter` _array_element)))

(event `self.ReceiveTick`
  (params (DeltaSeconds :type "Float (single-precision)"))
  (`self.K2_SetActorLocation` (`KismetMathLibrary.VInterpTo` (`self.K2_GetActorLocation`) (`/Game/Game/Blueprint/Player/PlayerCharacter.RewindCurrentLocation` (`self.PlayerCharacter`)) (`GameplayStatics.GetWorldDeltaSeconds`) 4.0))
  (set `self.Time` (+ (`GameplayStatics.GetWorldDeltaSeconds`) (`self.Time`)))
  (`self.K2_SetActorRotation` (`KismetMathLibrary.MakeRotator` (* (`self.Time`) 20.0) (* (`self.Time`) 100.0) (`self.Time`))))

(fn `UserConstructionScript`)