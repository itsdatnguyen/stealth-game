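; BP_CharacterInterface appears to be a Blueprint interface that defines a shared set of calls on game characters, with only default-value stubs here.
; Its queries cover visibility and location for an actor, state, last seen location, character reference and a timer.
; Other calls set maximum or minimum movement, report projectile hits with a hit value, and check for kills from an impact normal and location.
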(fn `CheckForKill`
  (params (`Impact Normal` :type "Vector Structure") (`Impact Location` :type "Vector Structure"))
  (returns (NewParam :type Boolean))
  (return false))

(fn `Get Character Reference`
  (returns (`Actor Reference` :type "Pawn Object Reference"))
  (return null))

(fn `Get Last Seen Location`
  (returns (`Last Seen Location` :type "Vector Structure"))
  (return (0.0 0.0 0.0)))

(fn `Get Location`
  (params (Actor :type "Actor Object Reference"))
  (returns (Lcoation :type "Vector Structure"))
  (return (0.0 0.0 0.0)))

(fn `Get State`
  (returns (Touched :type Boolean))
  (return false))

(fn `Get Timer`
  (returns (Time :type "Float (double-precision)"))
  (return 0.0))

(fn `Get Visibility`
  (params (Actor :type "Actor Object Reference"))
  (returns (`Visibility Value` :type "Float (double-precision)"))
  (return 0.0))

(fn `HitByProjectile`
  (params (`Hit Value` :type "Float (double-precision)"))
  (returns (NewParam1 :type "Float (double-precision)"))
  (return 0.0))

(fn `Set Move Max`
  (returns (NewParam :type Boolean))
  (return false))

(fn `Set Move Min`
  (returns (NewParam :type Boolean))
  (return false))