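; Game mode that tracks the player's last known position and runs timed enemy reinforcements.
; BeginPlay caches the player and enemy entry points; a flag lets Tick snapshot the player's location on request.
; Once activated, Tick accumulates time and, at each interval, shuffles the entries and spawns a basic enemy from the first.
; Separate functions store a ghost transform and replace the last-known-position indicator actor there.
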(event `self.ReceiveBeginPlay`
  (bind _outactors (`GameplayStatics.GetAllActorsOfClass` "/Game/Game/Blueprint/Player/PlayerCharacter.PlayerCharacter_C"))
  (for _array_element _outactors
    (set `self.Player` _array_element)
    (bind _outactors_2 (`GameplayStatics.GetAllActorsOfClass` "/Game/Game/Blueprint/BT_Enemy_Entry.BT_Enemy_Entry_C"))
    (set `self.EnemyEntry` _outactors_2)
    (`self.SetLastKnownPosition`)))

(event `self.ReceiveTick`
  (params (DeltaSeconds :type "Float (single-precision)"))
  (bind _enemyentry (`self.EnemyEntry`))
  (if (`self.SetLastKnownPositionFlag`)
    (`self.SetLastKnownPosition`))
  (if (`self.Activated`)
    (set `self.TimeElapsed` (+ (`GameplayStatics.GetWorldDeltaSeconds`) (`self.TimeElapsed`)))
    (if (>= (/ (`self.TimeElapsed`) (* (`self.EventIntervalLength`) (`self.PenaltyNumber`))) 1.0)
      (set `self.PenaltyNumber` (+ (`self.PenaltyNumber`) 1.0))
      (`KismetArrayLibrary.Array_Shuffle` _enemyentry)
      (`/Game/Game/Blueprint/BT_Enemy_Entry.SpawnBasicEnemy` (`KismetArrayLibrary.Array_Get` _enemyentry)))))

(fn `ActivateReinforcements`
  (returns (Null :type Boolean))
  (set `self.Activated` true)
  (return false))

(fn `GetLastKnownPosition`
  (returns (PlayerLastKnownPosition :type "Vector Structure"))
  (return (`self.PlayerLastKnownPosition`)))

(fn `SetGhostIndicator`
  (if (not (== (`self.LastKnownPosition`) null))
    (`self.K2_DestroyActor` (`self.LastKnownPosition`)))
  (bind _returnvalue (`|SpawnActorFromClass` "/Game/Game/Blueprint/BT_LastKnownPosition.BT_LastKnownPosition_C" (`KismetMathLibrary.MakeTransform` (`self.GhostLocation`) (`self.GhostRotation`) (0.9 0.9 0.9)) "AdjustIfPossibleButDontSpawnIfColliding" "OverrideRootScale"))
  (set `self.LastKnownPosition` _returnvalue)
  (return))

(fn `SetGhostParameters`
  (params (GhostLocation :type "Vector Structure") (GhostRotation :type "Rotator Structure"))
  (set `self.GhostLocation` GhostLocation)
  (set `self.GhostRotation` GhostRotation))

(fn `SetLastKnownPosition`
  (set `self.PlayerLastKnownPosition` (`self.K2_GetActorLocation` (`self.Player`)))
  (set `self.SetLastKnownPositionFlag` false))

(fn `SetLastKnownPositionFlagTrue`
  (set `self.SetLastKnownPositionFlag` true))

(fn `UserConstructionScript`)