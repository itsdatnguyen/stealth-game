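; Key-locked door that opens when the player runs into it while any of its assigned keys is activated.
; Opening hides the cube and disables its collision; construction sets its scale, rotation, mesh and material from variables.
; Each activated key found on hit also alerts all CH_BasicEnemy actors: the game mode's last known position is set and enemies are flagged to move there, with unaware ones also calling AlertTimer.
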(event `self.ReceiveHit`
  (params (MyComp :type "PrimitiveComponent Object Reference") (Other :type "Actor Object Reference") (OtherComp :type "PrimitiveComponent Object Reference") (bSelfMoved :type Boolean) (HitLocation :type "Vector Structure") (HitNormal :type "Vector Structure") (NormalImpulse :type "Vector Structure") (Hit :type "HitResult Structure (by ref)"))
  (bind _asgame_mode (cast `/Game/Game/Blueprint/Statics/Game_Mode` (`GameplayStatics.GetGameMode`) :!pure true))
  (if (== (`GameplayStatics.GetObjectClass` Other) "/Game/Game/Blueprint/Player/PlayerCharacter.PlayerCharacter_C")
    (for _array_element (`self.Keys`)
      (bind _activated (`/Game/Game/Blueprint/BP_DoorKey.GetActivated` _array_element))
      (if _activated
        (`self.OpenGate`)
        (bind _outactors (`GameplayStatics.GetAllActorsOfClass` "/Game/Game/Blueprint/Enemy/CH_BasicEnemy.CH_BasicEnemy_C"))
        (for _array_element_2 _outactors
          (bind _service (`/Game/Game/Blueprint/Enemy/CH_BasicEnemy.GetService` _array_element_2))
          (bind (_aggressive _aware) (`/Game/Game/Blueprint/Enemy/AI/TasksInUse/BP_BasicEnemyService.GetState` _service))
          (if _aware
            (`/Game/Game/Blueprint/Statics/Game_Mode.SetLastKnownPosition` _asgame_mode)
            (`/Game/Game/Blueprint/Enemy/AI/TasksInUse/BP_BasicEnemyService.SetFlagMoveToLastKnownLocation` _service)
            (else
              (`/Game/Game/Blueprint/Enemy/AI/TasksInUse/BP_BasicEnemyService.AlertTimer` _service)
              (`/Game/Game/Blueprint/Statics/Game_Mode.SetLastKnownPosition` _asgame_mode)
              (`/Game/Game/Blueprint/Enemy/AI/TasksInUse/BP_BasicEnemyService.SetFlagMoveToLastKnownLocation` _service))))))))

(fn `AssignToDoor`
  (params (Key :type "/Game/Game/Blueprint/BP_DoorKey Object Reference"))
  (`KismetArrayLibrary.Array_Add` (`self.Keys`) Key))

(fn `OpenGate`
  (bind _cube (`self.Cube`))
  (`SceneComponent.SetVisibility` _cube false false)
  (`PrimitiveComponent.SetCollisionEnabled` _cube "NoCollision"))

(fn `UserConstructionScript`
  (`SceneComponent.SetWorldScale3D` (`self.Cube`) (`self.CubeScale`))
  (`SceneComponent.K2_SetWorldRotation` (`self.Cube`) (`self.CubeRotation`) false false)
  (`StaticMeshComponent.SetStaticMesh` (`self.Cube`) (`self.StaticMesh`))
  (`PrimitiveComponent.CreateDynamicMaterialInstance` (`self.Cube`) 0 (`self.Material`)))